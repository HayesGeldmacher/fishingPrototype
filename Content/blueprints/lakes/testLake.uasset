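; Test lake for a fishing mechanic that spawns fish and responds to catches.
; spawnFish waits a random delay, then spawns a random class from Fishies at the given point and sets FishCurrent to block further spawns.
; Tick prints debug text while a fish is current.
; FishCaught prints and clears BobOut on the first-person character but leaves FishCurrent set.
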(event Custom|spawnFish
  (params (SpawnPoint :type Vector))
  (bind _fishies (Variables|Default|GetFishies))
  (if (not (Variables|Default|GetFishCurrent))
    (Utilities|FlowControl|Delay (Math|Random|RandomFloatinRange (Variables|Default|GetminSpawnTime) (Variables|Default|GetMaxSpawnTime)))
    (bind _output_get (Variables|Default|SetspawnNum (Math|Random|RandomInteger (Utilities|Array|Length _fishies))))
    (Game|SpawnActorfromClass (Utilities|Array|Get(acopy) _fishies _output_get) (Math|Transform|MakeTransform SpawnPoint "0, 0, 0" "1.000000,1.000000,1.000000") "Undefined" "MultiplyWithRoot" 0 0)
    (Variables|Default|SetFishCurrent true)))

(event Custom|FishCaught
  (params (NewParam :type Actor%20Class%20Reference))
  (Development|PrintString "fishCaught!")
  (bind _returnvalue (Actor|GetActorOfClass "/Game/FirstPerson/Blueprints/BP_FirstPersonCharacter.BP_FirstPersonCharacter_C"))
  (Variables|/Game/FirstPerson/Blueprints/BP_FirstPersonCharacter.BP_FirstPersonCharacter_C|SetbobOut _returnvalue false))

(event EventBeginPlay)

(event Collision|EventActorBeginOverlap
  (params (OtherActor :type Actor%20Object%20Reference)))

(event EventTick
  (params (DeltaSeconds :type Float%20%28single-precision%29))
  (if (Variables|Default|GetFishCurrent)
    (Development|PrintString "fishMoving! 
")))

(fn ConstructionScript)