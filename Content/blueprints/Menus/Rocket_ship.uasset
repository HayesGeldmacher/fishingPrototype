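; Rocket_ship is an actor that the player moves with the W, A, S and D keys.
; Key press and release events set held-state flags, which Tick turns into forward/back and left/right offsets of Speed, with W and A taking priority over their opposites.
; AddActorLocalOffset applies the movement relative to the actor's rotation every frame, without delta-time scaling, so travel speed depends on frame rate.
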(event EventTick
  (params (DeltaSeconds :type Float%20%28single-precision%29))
  (bind _speed (Variables|Default|Getspeed))
  (bind _speed_2 (Variables|Default|Getspeed))
  (if (Variables|Default|GetWDown)
    (Variables|Default|SetXDirection _speed_2)
    (elif (Variables|Default|GetSDown)
      (Variables|Default|SetXDirection (* _speed_2 -1.0))
      (else
        (Variables|Default|SetXDirection 0.0))))
  (if (Variables|Default|GetADown)
    (Variables|Default|SetYDirection (* _speed -1.0))
    (elif (Variables|Default|GetDDown)
      (Variables|Default|SetYDirection _speed)
      (else
        (Variables|Default|SetYDirection 0.0))))
  (Transformation|AddActorLocalOffset (Math|Vector|MakeVector (Variables|Default|GetXDirection) (Variables|Default|GetYDirection) 0.0) false false))

(event Input|KeyboardEvents|W
  (params (Key :type Key%20Structure :default "None"))
  ;[1 1 1] checks for input
  (:Pressed
    (Variables|Default|SetWDown true))
  (:Released
    (Variables|Default|SetWDown false)))

(event Input|KeyboardEvents|S
  (params (Key :type Key%20Structure :default "None"))
  ;[1 1 1] checks for input
  (:Pressed
    (Variables|Default|SetSDown true))
  (:Released
    (Variables|Default|SetSDown false)))

(event Input|KeyboardEvents|A
  (params (Key :type Key%20Structure :default "None"))
  ;[1 1 1] checks for input
  (:Pressed
    (Variables|Default|SetADown true))
  (:Released
    (Variables|Default|SetADown false)))

(event Input|KeyboardEvents|D
  (params (Key :type Key%20Structure :default "None"))
  ;[1 1 1] checks for input
  (:Pressed
    (Variables|Default|SetDDown true))
  (:Released
    (Variables|Default|SetDDown false)))

(fn ConstructionScript)