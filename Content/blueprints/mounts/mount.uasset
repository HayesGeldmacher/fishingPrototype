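; Fish mount Blueprint that displays its fish mesh only if that fish is recorded as caught.
; On BeginPlay it casts the game instance to GameManage and looks up its Fish variable in the CatchList map.
; A value of 1 shows FishMesh and any other value hides it, with debug prints along the way.
; The check runs only once, at BeginPlay.
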(event EventBeginPlay
  (Development|PrintString "mount")
  (bind _asgame_manage (Utilities|Casting|CastToGameManage (Game|GetGameInstance)))
  (if (== (.Value (Utilities|Map|Find (Variables|/Game/blueprints/GameManage.GameManage_C|GetCatchList _asgame_manage) (Variables|Default|Getfish))) 1)
    (Development|PrintString "succeeded")
    (Rendering|SetVisibility (Variables|Default|GetfishMesh) true false)
    (else
      (Development|PrintString "failed")
      (Rendering|SetVisibility (Variables|Default|GetfishMesh) false false))))

(fn ConstructionScript)