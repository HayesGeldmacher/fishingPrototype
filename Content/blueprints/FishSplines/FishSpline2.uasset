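; Fish actor for a fishing game that swims along a spline each tick, optionally looping, with a yaw offset.
; The caughtFish event resets the first-person character's ReelPower, speeds up the fish and starts a looping five-second check timer.
; If ReelPower exceeds MinReelPower at a check, the fish snaps to the character's SpawnPoint and is destroyed after a delay.
; Otherwise it returns to uncaught swimming.
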(event Custom|caughtFish
  (Variables|Default|SetisCaught true)
  (bind _returnvalue (Actor|GetActorOfClass "/Game/FirstPerson/Blueprints/BP_FirstPersonCharacter.BP_FirstPersonCharacter_C"))
  (Variables|/Game/FirstPerson/Blueprints/BP_FirstPersonCharacter.BP_FirstPersonCharacter_C|SetreelPower _returnvalue 0.0))

(event Custom|test
  (bind _returnvalue (Actor|GetActorOfClass "/Game/FirstPerson/Blueprints/BP_FirstPersonCharacter.BP_FirstPersonCharacter_C"))
  (if (> (Variables|/Game/FirstPerson/Blueprints/BP_FirstPersonCharacter.BP_FirstPersonCharacter_C|GetreelPower _returnvalue) (Variables|Default|GetminReelPower))
    (Variables|/Game/FirstPerson/Blueprints/BP_FirstPersonCharacter.BP_FirstPersonCharacter_C|SetreelPower _returnvalue 0.0)
    (Variables|Default|Setisdefeated true)
    (else
      (Variables|Default|SetisCaught false)
      (Variables|Default|SettimerisStarted false))))

(event EventBeginPlay)

(event Collision|EventActorBeginOverlap
  (params (OtherActor :type Actor%20Object%20Reference)))

(event EventTick
  (params (DeltaSeconds :type Float%20%28single-precision%29))
  (bind _relativescale3d (Variables|Default|GetRelativeScale3D))
  (if (Variables|Default|GetisCaught)
    (Variables|Default|SetSpeed 6e+02)
    (if (Variables|Default|GettimerisStarted)
      _
      (else
        (Utilities|Time|SetTimerbyEvent (delegate Custom|test) 5.0 true)
        (Variables|Default|SettimerisStarted true)))
    (else
      (Variables|Default|SetSpeed 3e+02)))
  (Variables|Default|SetDistanceSpline (+ (* DeltaSeconds (Variables|Default|GetSpeed)) (Variables|Default|GetDistanceSpline)))
  (if (Variables|Default|Getisdefeated)
    (Transformation|SetWorldTransform (Math|Transform|MakeTransform (Transformation|GetWorldLocation (Variables|/Game/FirstPerson/Blueprints/BP_FirstPersonCharacter.BP_FirstPersonCharacter_C|GetspawnPoint (stale Custom|test _returnvalue))) "0, 0, 0" _relativescale3d) false false)
    (Development|PrintString "Caught a Fish!")
    (Utilities|FlowControl|Delay 3.0)
    (Actor|DestroyActor)
    (else
      (Transformation|SetRelativeTransform (Math|Transform|MakeTransform (Math|Vector|MakeVector (.x (.location (Spline|GetTransformatDistanceAlongSpline (Variables|Default|GetSpline) (Variables|Default|GetDistanceSpline) "Local" false))) (.y (.location (Spline|GetTransformatDistanceAlongSpline (Variables|Default|GetSpline) (Variables|Default|GetDistanceSpline) "Local" false))) (.z (.location (Spline|GetTransformatDistanceAlongSpline (Variables|Default|GetSpline) (Variables|Default|GetDistanceSpline) "Local" false)))) (Math|Rotator|MakeRotator (.roll (.rotation (Spline|GetTransformatDistanceAlongSpline (Variables|Default|GetSpline) (Variables|Default|GetDistanceSpline) "Local" false))) (.pitch (.rotation (Spline|GetTransformatDistanceAlongSpline (Variables|Default|GetSpline) (Variables|Default|GetDistanceSpline) "Local" false))) (- (.yaw (.rotation (Spline|GetTransformatDistanceAlongSpline (Variables|Default|GetSpline) (Variables|Default|GetDistanceSpline) "Local" false))) 9e+01)) _relativescale3d) false false)
      (if (Variables|Default|Getloop)
        (if (> (Variables|Default|GetDistanceSpline) (Spline|GetSplineLength (Variables|Default|GetSpline)))
          (Variables|Default|SetDistanceSpline 0.0))))))

(fn ConstructionScript)

(fn FishWiggle
  (Variables|Default|SetisCaught false)
  (Development|PrintString "fishNotWiggle! 
")
  (Variables|Default|SettimerisStarted false)
  (Actor|DestroyActor))