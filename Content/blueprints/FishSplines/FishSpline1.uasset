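; FishSpline1 is an actor that moves its Character component, presumably a fish, along its Spline.
; Each Tick advances a distance by Speed times delta time and applies the spline's local transform at that point to Character.
; A yaw offset corrects the facing, and the component keeps its own scale.
; With Loop set, the distance resets to zero past the spline's end.
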(event EventBeginPlay)

(event Collision|EventActorBeginOverlap
  (params (OtherActor :type Actor%20Object%20Reference)))

(event EventTick
  (params (DeltaSeconds :type Float%20%28single-precision%29))
  (Variables|Default|SetDistanceSpline (+ (* DeltaSeconds (Variables|Default|GetSpeed)) (Variables|Default|GetDistanceSpline)))
  (Transformation|SetRelativeTransform (Variables|Default|Getcharacter) (Math|Transform|MakeTransform (Math|Vector|MakeVector (.x (.location (Spline|GetTransformatDistanceAlongSpline (Variables|Default|GetSpline) (Variables|Default|GetDistanceSpline) "Local" false))) (.y (.location (Spline|GetTransformatDistanceAlongSpline (Variables|Default|GetSpline) (Variables|Default|GetDistanceSpline) "Local" false))) (.z (.location (Spline|GetTransformatDistanceAlongSpline (Variables|Default|GetSpline) (Variables|Default|GetDistanceSpline) "Local" false)))) (Math|Rotator|MakeRotator (.roll (.rotation (Spline|GetTransformatDistanceAlongSpline (Variables|Default|GetSpline) (Variables|Default|GetDistanceSpline) "Local" false))) (.pitch (.rotation (Spline|GetTransformatDistanceAlongSpline (Variables|Default|GetSpline) (Variables|Default|GetDistanceSpline) "Local" false))) (- (.yaw (.rotation (Spline|GetTransformatDistanceAlongSpline (Variables|Default|GetSpline) (Variables|Default|GetDistanceSpline) "Local" false))) 9e+01)) (Variables|/Script/Engine.SceneComponent|GetRelativeScale3D (Variables|Default|Getcharacter))) false false)
  (if (Variables|Default|Getloop)
    (if (> (Variables|Default|GetDistanceSpline) (Spline|GetSplineLength (Variables|Default|GetSpline)))
      (Variables|Default|SetDistanceSpline 0.0))))

(fn ConstructionScript)